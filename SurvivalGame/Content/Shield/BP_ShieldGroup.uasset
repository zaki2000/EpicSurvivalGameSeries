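; BP_ShieldGroup tracks a set of shields belonging to a parent pawn and reports when all of them are broken.
; On each shield-broken event it scans for any shield with health left, and if none remains it prints a message and notifies the pawn.
; CanDamage always allows damage, and a direct-kill call on the pawn is present but never runs.
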(event Custom|CustomEvent_OnShield_broken
  (params (DamageType :type Damage%20Type%20Object%20Reference) (Instigator :type Controller%20Object%20Reference) (DamageCauser :type Actor%20Object%20Reference))
  (Variables|Default|SetShieldCount 0)
  (bind _array_element (Utilities|Array|ForEachLoopwithBreak (Variables|Default|GetShields) :!label _label)
    (:LoopBody
      (if (> (Variables|/Game/Shield/BP_Shield.BP_Shield_C|GetHealth _array_element) 0.0)
        (Math|Integer|IncrementInt (Variables|Default|GetShieldCount)
          (:%20%20
            (goto _label Break)))))
    (:Completed
      (if (== (Variables|Default|GetShieldCount) 0)
        (Development|PrintString "all shield is broken")
        (Class|SBaseCharacter|OnEventAllShieldsBroken (Variables|Default|GetParentPawn))))))

(event EventBeginPlay)

(event EventTick
  (params (DeltaSeconds :type Float%20%28single-precision%29)))

(fn CanDamage
  (params (DamagedObject :type BP%20Shield%20Object%20Reference))
  (return true))