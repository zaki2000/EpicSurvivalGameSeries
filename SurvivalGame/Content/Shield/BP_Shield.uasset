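; BP_Shield is a damageable shield actor that belongs to a parent group and can be broken.
; On any damage, it asks the group whether it can be damaged, then checks the damage type class before subtracting from Health.
; When Health runs out, it notifies the group that the shield broke, hides its collision component and children, and disables actor collision instead of destroying itself.
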(event EventBeginPlay)

(event Collision|EventActorBeginOverlap
  (params (OtherActor :type Actor%20Object%20Reference)))

(event EventTick
  (params (DeltaSeconds :type Float%20%28single-precision%29)))

(event Game|Damage|EventAnyDamage
  (params (Damage :type Float%20%28single-precision%29) (DamageType :type Damage%20Type%20Object%20Reference) (InstigatedBy :type Controller%20Object%20Reference) (DamageCauser :type Actor%20Object%20Reference))
  (bind _result (Default|CanDamage (Variables|Default|GetParentGroup) self))
  (if _result
    (if (== (Utilities|GetClass DamageType) (Variables|Default|GetDamageType))
      (bind _output_get (Variables|Default|SetHealth (- (Variables|Default|GetHealth) Damage)))
      (if (<= _output_get 0.0)
        (Default|CustomEventonShieldBroken (Variables|Default|GetParentGroup))
        (Rendering|SetVisibility (Variables|Default|GetCollisionComponent) false true)
        (Collision|SetActorEnableCollision self false)))))

(fn ConstructionScript)