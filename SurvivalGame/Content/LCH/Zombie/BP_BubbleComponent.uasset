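; BP_BubbleComponent is a widget component that displays a text bubble for its owning actor.
; On BeginPlay, outside dedicated servers, it casts its widget to UW_Bubble, caches it and prints the owner's name.
; SetBubbleText forwards a value to that cached widget without a validity check.
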(event EventBeginPlay
  (if (not (Networking|IsDedicatedServer))
    (bind _asuw_bubble (Utilities|Casting|CastToUW_Bubble (UserInterface|GetUserWidgetObject)))
    (Variables|Default|SetUW_BubbleText _asuw_bubble)
    (Development|PrintString (Utilities|GetObjectName (Components|GetOwner)))))

(fn SetBubbleText
  (params (Value :type String))
  (Default|SetBubbleTextValue (Variables|Default|GetUW_BubbleText) Value))