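; Zombie NPC Blueprint that stays dormant until the game level reaches its own, then senses pawns and talks through an overhead bubble.
; On the dedicated server, BeginPlay disables sensing and binds to the game mode's level-change event, which re-enables it and triggers talk.
; While firing, Tick repeats the skill component's normal attack at a fixed interval.
; Dialogue steps through talk sections on a timer, then restores the NPC name.
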(event Custom|TalkInClient
  (CallFunction|StartTalk))

(event Custom|OnGameModeLevelChanged
  (params (NewLevel :type Integer))
  (if (>= NewLevel (Variables|Default|GetLevel))
    (CallFunction|SetNPCActive true)))

(event EventBeginPlay
  (|CallParentFunction)
  (if (Networking|IsDedicatedServer)
    (CallFunction|SetBubbleTextValue (Variables|Default|GetNPCName))
    (CallFunction|SetNPCActive false)
    (bind _asnew_game_mode (Utilities|Casting|CastToNewGameMode (Game|GetGameMode)))
    (EventDispatchers|BindEventtoOnServerLevelChanged _asnew_game_mode (delegate Custom|OnGameModeLevelChanged))))

(event EventTick
  (params (DeltaSeconds :type Float%20%28single-precision%29))
  (if (Variables|Default|GetIsFiring)
    (Variables|Default|SetCurrentSkillUseDeltaTime (+ (Variables|Default|GetCurrentSkillUseDeltaTime) DeltaSeconds))
    (while (>= (Variables|Default|GetCurrentSkillUseDeltaTime) (Variables|Default|GetCurrentSkillUseMaxInterval))
      (Variables|Default|SetCurrentSkillUseDeltaTime (- (Variables|Default|GetCurrentSkillUseDeltaTime) (Variables|Default|GetCurrentSkillUseMaxInterval)))
      (CallFunction|UseCurrentSkill))))

(fn ConstructionScript
  (|CallParentFunction))

(fn StartFire
  (Variables|Default|SetIsFiring true)
  (CallFunction|UseCurrentSkill)
  (Variables|Default|SetCurrentSkillUseDeltaTime 0.0))

(fn StopFire
  (Variables|Default|SetIsFiring false))

(fn UseCurrentSkill
  (if (== (Variables|Default|GetCurrentSkillIndex) 0)
    (Default|NormalAttack (Variables|Default|GetBP_ZombieSkillComponent) "0, 0, 0")))

(fn SetBubbleTextValue
  (params (Value :type String))
  (bind _asuw_bubble (Utilities|Casting|CastToUW_Bubble (UserInterface|GetUserWidgetObject (Variables|Default|GetBubble))))
  (Default|SetBubbleTextValue _asuw_bubble Value))

(fn TalkNextSection
  (bind _talksections (Variables|Default|GetTalkSections))
  (if (< (Variables|Default|GetCurrentSectionIndex) (Utilities|Array|Length _talksections))
    (CallFunction|SetBubbleTextValue (Utilities|Array|Get(acopy) _talksections (Variables|Default|GetCurrentSectionIndex)))
    (Math|Integer|IncrementInt (Variables|Default|GetCurrentSectionIndex)
      (:%20%20
        (Utilities|Time|SetTimerbyEvent (EventDispatchers|CreateEvent :!event TalkNextSection) (Variables|Default|GetTalkInterval))))
    (else
      (Variables|Default|SetTalking false)
      (CallFunction|SetBubbleTextValue (Variables|Default|GetNPCName)))))

(fn StartTalk
  (if (not (Variables|Default|GetTalking))
    (Variables|Default|SetCurrentSectionIndex 0)
    (CallFunction|TalkNextSection)))

(fn SetNPCActive
  (params (Active :type Boolean))
  (Class|PawnSensingComponent|SetSensingUpdatesEnabled (Variables|Default|GetPawnSensingComp) Active)
  (if Active
    (CallFunction|TalkinClient)))