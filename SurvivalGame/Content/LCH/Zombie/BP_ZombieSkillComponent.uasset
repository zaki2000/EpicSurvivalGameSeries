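; Zombie skill component that gives its owning BP_NewZombie a ranged attack, firing BP_Projectile with a rifle sound.
; NormalAttack takes the owner's transform or its projectile spawn point, adds look-at rotation when given a target, and makes projectiles ignore the owner.
; As written, targeted shots spawn at the world origin.
; RandomRotator builds its spread only from the random range, discarding the input aim rotation.
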(event EventBeginPlay
  (bind _asbp_new_zombie (Utilities|Casting|CastToBP_NewZombie (Components|GetOwner)))
  (bind _output_get (Variables|Default|SetOwnerZombie _asbp_new_zombie))
  (Variables|Default|SetFireSpawnTransform (Variables|/Game/LCH/Zombie/BP_NewZombie.BP_NewZombie_C|GetProjectileSpawnTransform _output_get)))

(fn NormalAttack
  (params (TargetLocation :type Vector))
  (if (Variables|Default|GetUseOwnerTransform)
    (LocalVariables|SettmpTransform (Transformation|GetActorTransform (Variables|Default|GetOwnerZombie)))
    (else
      (LocalVariables|SettmpTransform (Transformation|GetWorldTransform (Variables|Default|GetFireSpawnTransform)))))
  (if (Math|Vector|Equal(Vector) TargetLocation "0, 0, 0" 0.0001)
    ;[1 1 1] 直接用当前旋转方向发射子弹
    (bind _returnvalue (Game|SpawnActorfromClass "/Game/LCH/Zombie/BP_Projectile.BP_Projectile_C" (Math|Transform|MakeTransform (.Location (Math|Transform|BreakTransform (LocalVariables|GettmpTransform))) (CallFunction|RandomRotator (.Rotation (Math|Transform|BreakTransform (LocalVariables|GettmpTransform))) (Variables|Default|GetRandomRotation)) (.Scale (Math|Transform|BreakTransform (LocalVariables|GettmpTransform)))) "AlwaysSpawn" 0 0))
    (Utilities|Array|Add (Variables|/Game/LCH/Zombie/BP_Projectile.BP_Projectile_C|GetIgnoresActors _returnvalue) (Variables|Default|GetOwnerZombie))
    (Audio|PlaySoundatLocation "/Game/Sound/Weapons/AssaultRifle_Shot_Cue.AssaultRifle_Shot_Cue" (.Location (Math|Transform|BreakTransform (LocalVariables|GettmpTransform))))
    (else
      ;[1 1 1] 根据传入的目标位置，算出起始旋转方向，然后在发射子弹
      (bind _returnvalue_2 (Game|SpawnActorfromClass "/Game/LCH/Zombie/BP_Projectile.BP_Projectile_C" (Math|Transform|MakeTransform "0, 0, 0" (CallFunction|RandomRotator (Math|Rotator|CombineRotators (.Rotation (Math|Transform|BreakTransform (LocalVariables|GettmpTransform))) (Math|Rotator|FindLookatRotation (.Location (Math|Transform|BreakTransform (LocalVariables|GettmpTransform))) TargetLocation)) (Variables|Default|GetRandomRotation))) "AlwaysSpawn" 0 0))
      (Utilities|Array|Add (Variables|/Game/LCH/Zombie/BP_Projectile.BP_Projectile_C|GetIgnoresActors _returnvalue_2) (Variables|Default|GetOwnerZombie))
      (Audio|PlaySoundatLocation "/Game/Sound/Weapons/AssaultRifle_Shot_Cue.AssaultRifle_Shot_Cue" (Transformation|GetWorldLocation (Variables|Default|GetFireSpawnTransform))))))

(fn RandomRotator
  (params (Input :type Rotator) (Random :type Rotator))
  (bind (_roll _pitch _yaw) (Math|Rotator|BreakRotator Random))
  (bind _result (Math|Float|NegateFloat _roll)
    (:%20%20
      (bind _result_2 (Math|Float|NegateFloat _pitch)
        (:%20%20
          (bind _result_3 (Math|Float|NegateFloat _yaw)
            (:%20%20
              (return (Math|Rotator|MakeRotator (+ (Math|Random|RandomFloatinRange _result _roll) _roll) (+ (Math|Random|RandomFloatinRange _result_2 _pitch) _pitch) (+ (Math|Random|RandomFloatinRange _result_3 _yaw) _yaw))))))))))