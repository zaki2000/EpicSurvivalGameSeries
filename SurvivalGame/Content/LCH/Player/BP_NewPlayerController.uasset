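; BP_NewPlayerController is a player controller that manages match UI for countdown, game start, aiming and game end.
; On non-dedicated-server instances, BeginPlay creates hidden start and aim widgets, and Tick shows the aim widget while the controlled BP_NewPlayerPawn is targeting.
; Game events update the countdown, display the start state before a timer hides it, and lazily create the end widget to show the win result.
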(event Custom|OnUpdateGameStartCountingDown
  (params (RemainTime :type Float%20%28single-precision%29) (Visible :type Boolean))
  (Default|UpdateCountingDownInfo (Variables|Default|GetUIGameStart) RemainTime Visible))

(event Custom|CloseGameStartUI
  (Widget|SetVisibility (Variables|Default|GetUIGameStart) "Hidden"))

(event Custom|OnGameStart
  (Default|SetGameStart (Variables|Default|GetUIGameStart))
  (Utilities|Time|SetTimerbyEvent (delegate Custom|CloseGameStartUI) 2.0))

(event Custom|OnGameEnd
  (params (Win :type Boolean))
  (if (!= (Variables|Default|GetUIGameEnd) 0)
    _
    (else
      (bind _returnvalue (UserInterface|CreateWidget "/Game/LCH/UI/UW_GameEnd.UW_GameEnd_C" self))
      (UserInterface|Viewport|AddtoViewport _returnvalue 0)
      (bind _output_get (Variables|Default|SetUIGameEnd _returnvalue))))
  (Widget|SetVisibility _output_get "Visible")
  (Default|SetResult _output_get Win))

(event EventBeginPlay
  (bind _self self)
  (if (not (Networking|IsDedicatedServer))
    (Utilities|FlowControl|Sequence
      (:then_0
        (bind _returnvalue (UserInterface|CreateWidget "/Game/LCH/UI/UW_GameStart.UW_GameStart_C" _self))
        (UserInterface|Viewport|AddtoViewport _returnvalue 0)
        (bind _output_get (Variables|Default|SetUIGameStart _returnvalue))
        (Widget|SetVisibility _output_get "Hidden"))
      (:then_1
        (bind _returnvalue_2 (UserInterface|CreateWidget "/Game/LCH/UI/UW_Aim.UW_Aim_C" _self))
        (UserInterface|Viewport|AddtoViewport _returnvalue_2 0)
        (bind _output_get_2 (Variables|Default|SetUIAim _returnvalue_2))
        (Widget|SetVisibility _output_get_2 "Hidden")))))

(event EventTick
  (params (DeltaSeconds :type Float%20%28single-precision%29))
  (bind _uiaim (Variables|Default|GetUIAim))
  (if (not (Networking|IsDedicatedServer))
    (if (!= (Variables|Default|GetUIAim) 0)
      (bind _asbp_new_player_pawn (Utilities|Casting|CastToBP_NewPlayerPawn (Pawn|GetControlledPawn)))
      (if (Class|SBaseCharacter|IsTargeting _asbp_new_player_pawn)
        (Widget|SetVisibility _uiaim "Visible")
        (else
          (Widget|SetVisibility _uiaim "Hidden"))))))

(fn ConstructionScript)

(fn UpdateGameStartCountingDownInfo
  (params (RemainTime :type Float%20%28single-precision%29) (Visible :type Boolean)))

(fn SetGameStart)