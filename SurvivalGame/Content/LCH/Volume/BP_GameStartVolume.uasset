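; BP_GameStartVolume is a trigger volume that tracks which players are waiting to start the game, acting only on a dedicated server.
; On begin and end overlap, it searches all BP_NewPlayerController actors for the one whose controlled pawn is the overlapping actor.
; It then passes that controller to NewGameMode to add it to or remove it from the waiting-start players.
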(event Collision|EventActorBeginOverlap
  (params (OtherActor :type Actor%20Object%20Reference))
  (if (Networking|IsDedicatedServer)
    (CallFunction|AddStartPlayer OtherActor)))

(event Collision|EventActorEndOverlap
  (params (OtherActor :type Actor%20Object%20Reference))
  (if (Networking|IsDedicatedServer)
    (CallFunction|RemoveStartPlayer OtherActor)))

(event EventBeginPlay
  (if (Networking|IsDedicatedServer)
    (Utilities|Casting|CastToNewGameMode (Game|GetGameMode))))

(fn ConstructionScript)

(fn AddStartPlayer
  (params (Actor :type Actor%20Object%20Reference))
  (bind _outactors (Actor|GetAllActorsOfClass "/Game/LCH/Player/BP_NewPlayerController.BP_NewPlayerController_C"))
  (for _array_element _outactors
    (if (== (Pawn|GetControlledPawn _array_element) Actor)
      (bind _asnew_game_mode (Utilities|Casting|CastToNewGameMode (Game|GetGameMode)))
      (Default|AddWaitingStartPlayer _asnew_game_mode _array_element)
      (return)))
  (return))

(fn RemoveStartPlayer
  (params (Actor :type Actor%20Object%20Reference))
  (bind _outactors (Actor|GetAllActorsOfClass "/Game/LCH/Player/BP_NewPlayerController.BP_NewPlayerController_C"))
  (for _array_element _outactors
    (if (== (Pawn|GetControlledPawn _array_element) Actor)
      (bind _asnew_game_mode (Utilities|Casting|CastToNewGameMode (Game|GetGameMode)))
      (Default|RemoveWaitingStartPlayer _asnew_game_mode _array_element)
      (return)))
  (return))