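; BP_ZombieBoss is a zombie boss protected by two child-actor shields that fires its weapon when commanded to use its current skill.
; On BeginPlay it registers both armor shields with a shield group and makes its capsule and mesh ignore a custom trace channel.
; When all shields break, both block that channel again, and death destroys the armor components.
; The skill calls Fire on the child weapon toward the target location.
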(event EventOnEventDeath
  (Components|DestroyComponent (Variables|Default|GetArmorRight))
  (Components|DestroyComponent (Variables|Default|GetArmorLeft)))

(event EventBeginPlay
  (bind _bp_shieldgroup (Variables|Default|GetBP_ShieldGroup))
  (bind _bp_shieldgroup_2 (Variables|Default|GetBP_ShieldGroup))
  (bind _asbp_shield (Utilities|Casting|CastToBP_Shield (Variables|/Script/Engine.ChildActorComponent|GetChildActor (Variables|Default|GetArmorRight))))
  (Utilities|Array|Add (Variables|/Game/Shield/BP_ShieldGroup.BP_ShieldGroup_C|GetShields _bp_shieldgroup) _asbp_shield)
  (Variables|/Game/Shield/BP_Shield.BP_Shield_C|SetParentGroup _asbp_shield _bp_shieldgroup)
  (bind _asbp_shield_2 (Utilities|Casting|CastToBP_Shield (Variables|/Script/Engine.ChildActorComponent|GetChildActor (Variables|Default|GetArmorLeft))))
  (Utilities|Array|Add (Variables|/Game/Shield/BP_ShieldGroup.BP_ShieldGroup_C|GetShields _bp_shieldgroup_2) _asbp_shield_2)
  (Variables|/Game/Shield/BP_Shield.BP_Shield_C|SetParentGroup _asbp_shield_2 _bp_shieldgroup_2)
  (Variables|/Game/Shield/BP_ShieldGroup.BP_ShieldGroup_C|SetParentPawn (Variables|Default|GetBP_ShieldGroup) self)
  (Collision|SetCollisionResponsetoChannel (Variables|Default|GetCapsuleComponent) "ECC_GameTraceChannel1" "ECR_Ignore")
  (Collision|SetCollisionResponsetoChannel (Variables|Character|GetMesh) "ECC_GameTraceChannel1" "ECR_Ignore"))

(event EventOnEventAllShieldsBroken
  (Collision|SetCollisionResponsetoChannel (Variables|Default|GetCapsuleComponent) "ECC_GameTraceChannel1" "ECR_Block")
  (Collision|SetCollisionResponsetoChannel (Variables|Character|GetMesh) "ECC_GameTraceChannel1" "ECR_Block"))

(event EventOnCommondUseCurrentSkill
  (params (TargetLocation :type Vector%20%28by%20ref%29))
  (CallFunction|UseCurrentSkill TargetLocation))

(fn ConstructionScript
  (|CallParentFunction))

(fn UseCurrentSkill
  (params (TargetLocation :type Vector))
  (bind _self self)
  (bind _weapon (Variables|Default|GetWeapon))
  (bind _returnvalue (Transformation|GetActorTransform _self))
  (bind (_location _rotation) (Math|Transform|BreakTransform _returnvalue))
  (Utilities|IsValid _weapon
    (:Is%20Valid
      (bind _assweapon_base_bp (Utilities|Casting|CastToSWeaponBase_BP (Variables|/Script/Engine.ChildActorComponent|GetChildActor _weapon)))
      (Class|SWeaponBaseBP|Fire _assweapon_base_bp _location _rotation 0.0 TargetLocation))))