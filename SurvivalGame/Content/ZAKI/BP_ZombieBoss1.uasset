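; BP_ZombieBoss1 is a zombie boss protected by left and right armor shields.
; BeginPlay registers both child-actor shields with its shield group and makes the capsule and mesh ignore a custom collision channel (GameTraceChannel1).
; When all shields break, both components switch to blocking that channel, exposing the body to it.
; Skill commands pass their target location to a multicast fire event.
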(event Custom|CustomEvent_UpdateCollision
  (Collision|SetCollisionResponsetoChannel (Variables|Default|GetCapsuleComponent) "ECC_GameTraceChannel1" "ECR_Block")
  (Collision|SetCollisionResponsetoChannel (Variables|Character|GetMesh) "ECC_GameTraceChannel1" "ECR_Block"))

(event EventOnEventDeath)

(event EventBeginPlay
  (bind _bp_shieldgroup (Variables|Default|GetBP_ShieldGroup))
  (bind _bp_shieldgroup_2 (Variables|Default|GetBP_ShieldGroup))
  (|CallParentFunction)
  (bind _asbp_shield (Utilities|Casting|CastToBP_Shield (Variables|/Script/Engine.ChildActorComponent|GetChildActor (Variables|Default|GetArmorRight))))
  (Utilities|Array|Add (Variables|/Game/Shield/BP_ShieldGroup.BP_ShieldGroup_C|GetShields _bp_shieldgroup) _asbp_shield)
  (Variables|/Game/Shield/BP_Shield.BP_Shield_C|SetParentGroup _asbp_shield _bp_shieldgroup)
  (bind _asbp_shield_2 (Utilities|Casting|CastToBP_Shield (Variables|/Script/Engine.ChildActorComponent|GetChildActor (Variables|Default|GetArmorLeft))))
  (Utilities|Array|Add (Variables|/Game/Shield/BP_ShieldGroup.BP_ShieldGroup_C|GetShields _bp_shieldgroup_2) _asbp_shield_2)
  (Variables|/Game/Shield/BP_Shield.BP_Shield_C|SetParentGroup _asbp_shield_2 _bp_shieldgroup_2)
  (Variables|/Game/Shield/BP_ShieldGroup.BP_ShieldGroup_C|SetParentPawn (Variables|Default|GetBP_ShieldGroup) self)
  (Collision|SetCollisionResponsetoChannel (Variables|Default|GetCapsuleComponent) "ECC_GameTraceChannel1" "ECR_Ignore")
  (Collision|SetCollisionResponsetoChannel (Variables|Character|GetMesh) "ECC_GameTraceChannel1" "ECR_Ignore"))

(event EventOnEventAllShieldsBroken
  (CallFunction|CustomEventUpdateCollision))

(event EventOnCommondUseCurrentSkill
  (params (TargetLocation :type Vector%20%28by%20ref%29))
  (CallFunction|CustomEventMultiCastFire TargetLocation))

(fn ConstructionScript
  (|CallParentFunction))