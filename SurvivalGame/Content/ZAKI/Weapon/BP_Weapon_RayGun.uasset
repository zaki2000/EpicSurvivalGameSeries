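; BP_Weapon_RayGun is a hitscan weapon with a Fire event meant to shoot toward a target location or along a rotator.
; The location path line-traces on Visibility, ignoring the owning pawn, and applies point damage to the hit actor.
; A hard-coded false disables that path, so Fire always calls the rotator function, which is empty here.
; A helper adds random spread to a rotator but is not called in this file.
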(event EventBeginPlay)

(event Collision|EventActorBeginOverlap
  (params (OtherActor :type Actor%20Object%20Reference)))

(event EventFire
  (params (FromLocation :type Vector%20%28by%20ref%29) (Rotator :type Rotator%20%28by%20ref%29) (Range :type Float%20%28single-precision%29) (TargetLocation :type Vector%20%28by%20ref%29))
  (if (and false (Math|Vector|NotEqual(Vector) TargetLocation "0, 0, 0" 0.0001))
    (CallFunction|FireOncebyLocation FromLocation TargetLocation)
    (else
      (CallFunction|FireOncebyRotator FromLocation Rotator Range))))

(event EventTick
  (params (DeltaSeconds :type Float%20%28single-precision%29)))

(fn ConstructionScript)

(fn RandomFireRotator
  (params (Input :type Rotator) (Random :type Rotator))
  (bind (_roll _pitch _yaw) (Math|Rotator|BreakRotator Random))
  (bind (_roll_2 _pitch_2 _yaw_2) (Math|Rotator|BreakRotator Input))
  (if (Math|Rotator|Equal(Rotator) Random "0, 0, 0" 0.0001)
    (return Input)
    (else
      (bind _result (Math|Float|NegateFloat _roll)
        (:%20%20
          (bind _result_2 (Math|Float|NegateFloat _pitch)
            (:%20%20
              (bind _result_3 (Math|Float|NegateFloat _yaw)
                (:%20%20
                  (return (Math|Rotator|MakeRotator (+ (Math|Random|RandomFloatinRange _result _roll) _roll_2) (+ (Math|Random|RandomFloatinRange _result_2 _pitch) _pitch_2) (+ (Math|Random|RandomFloatinRange _result_3 _yaw) _yaw_2))))))))))))

(fn FireOncebyLocation
  (params (FromLocation :type Vector) (TargetLocation :type Vector))
  (bind _ignores (LocalVariables|GetIgnores))
  (bind _ownerpawn (Variables|Default|GetOwnerPawn))
  (if (Math|Vector|Equal(Vector) FromLocation "0, 0, 0" 0.0001)
    (LocalVariables|SetSrcLocation (Transformation|GetWorldLocation (Variables|Default|GetArrow)))
    (else
      (LocalVariables|SetSrcLocation FromLocation)))
  (Utilities|Array|Add _ignores (Variables|Default|GetOwnerPawn))
  (bind (_outhit _returnvalue) (Collision|LineTraceByChannel (LocalVariables|GetSrcLocation) TargetLocation "TraceTypeQuery1" false _ignores "None"))
  (if _returnvalue
    (Utilities|IsValid (.HitActor (Collision|BreakHitResult _outhit))
      (:Is%20Valid
        (Game|Damage|ApplyPointDamage (.HitActor (Collision|BreakHitResult _outhit)) (Variables|Default|GetDamage) (.Location (Collision|BreakHitResult _outhit)) _outhit (Pawn|GetController _ownerpawn) _ownerpawn "/Game/ZAKI/Weapon/Custom_DamageType1.Custom_DamageType1_C")))))

(fn FireOncebyRotator
  (params (FromLocation :type Vector) (Rotator :type Rotator) (Range :type Float%20%28single-precision%29)))