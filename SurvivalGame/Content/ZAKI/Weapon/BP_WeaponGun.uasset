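; Weapon gun Blueprint that fires projectiles, rate-limited by a minimum interval between shots.
; FireOncebyLocation starts at the given location or, if zero, the Arrow component, and aims at the target or, if zero, along the start rotation.
; It adds random spread, spawns ProjectileClass with the owner pawn as instigator, then sets the next allowed shot time.
; FireOncebyRotator is empty, and the shot sound nodes are unconnected.
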(event EventBeginPlay)

(event Collision|EventActorBeginOverlap
  (params (OtherActor :type Actor%20Object%20Reference)))

(event EventTick
  (params (DeltaSeconds :type Float%20%28single-precision%29)))

(event EventFireOncebyRotator
  (params (FromLocation :type Vector) (Rotator :type Rotator :default "0, 0, 0") (Range :type Float%20%28single-precision%29)))

(event EventFireOncebyLocation
  (params (FromLocation :type Vector) (TargetLocation :type Vector))
  (bind _output_get (Variables|Default|SettmNow (Math|DateTime|Now)))
  (if (>= _output_get (Variables|Default|GetShootTick))
    (if (Math|Vector|Equal(Vector) FromLocation "0, 0, 0" 0.0001)
      (Variables|Default|SettmpTransform (Transformation|GetWorldTransform (Variables|Default|GetArrow)))
      (else
        (Variables|Default|SettmpTransform (Math|Transform|MakeTransform FromLocation (Math|Rotator|FindLookatRotation FromLocation TargetLocation)))))
    (if (Math|Vector|Equal(Vector) TargetLocation "0, 0, 0" 0.0001)
      ;[1 1 1] 直接用当前旋转方向发射子弹
      (Game|SpawnActorfromClass (Variables|Default|GetProjectileClass) (Math|Transform|MakeTransform (.Location (Math|Transform|BreakTransform (Variables|Default|GettmpTransform))) (CallFunction|RandomFireRotator (.Rotation (Math|Transform|BreakTransform (Variables|Default|GettmpTransform))) (Variables|Default|GetRandomRotation)) (.Scale (Math|Transform|BreakTransform (Variables|Default|GettmpTransform)))) "AlwaysSpawn" self (Variables|Default|GetOwnerPawn))
      (Variables|Default|SetShootTick (+ (Variables|Default|GettmNow) (Math|Timespan|MakeTimespan 0 0 0 0 (Variables|Default|GetMinShootInterval_MS))))
      (else
        ;[1 1 1] 根据传入的目标位置，算出起始旋转方向，然后在发射子弹
        (Game|SpawnActorfromClass (Variables|Default|GetProjectileClass) (Math|Transform|MakeTransform (.Location (Math|Transform|BreakTransform (Variables|Default|GettmpTransform))) (CallFunction|RandomFireRotator (Math|Rotator|FindLookatRotation (.Location (Math|Transform|BreakTransform (Variables|Default|GettmpTransform))) TargetLocation) (Variables|Default|GetRandomRotation)) (.Scale (Math|Transform|BreakTransform (Variables|Default|GettmpTransform)))) "AlwaysSpawn" self (Variables|Default|GetOwnerPawn))
        (Variables|Default|SetShootTick (+ (Variables|Default|GettmNow) (Math|Timespan|MakeTimespan 0 0 0 0 (Variables|Default|GetMinShootInterval_MS))))))))

(fn ConstructionScript
  (|CallParentFunction))