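; Projectile gun weapon actor that spawns a projectile when Fire is called, rate-limited by a timestamp and a millisecond shoot interval.
; A zero FromLocation falls back to the Arrow component's transform, and a non-zero TargetLocation aims the shot at that point.
; Projectile class and interval come from getters, and each projectile receives the gun as Owner along with its Instigator.
; The gunshot sound nodes are disconnected, so firing plays no sound here.
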(event EventBeginPlay)

(event Collision|EventActorBeginOverlap
  (params (OtherActor :type Actor%20Object%20Reference)))

(event EventTick
  (params (DeltaSeconds :type Float%20%28single-precision%29)))

(event EventFire
  (params (FromLocation :type Vector%20%28by%20ref%29) (Rotator :type Rotator%20%28by%20ref%29 :default "0, 0, 0") (Range :type Float%20%28single-precision%29) (TargetLocation :type Vector%20%28by%20ref%29))
  (bind _output_get (Variables|Default|SettmNow (Math|DateTime|Now)))
  (if (>= _output_get (Variables|Default|GetShootTick))
    (if (Math|Vector|Equal(Vector) FromLocation "0, 0, 0" 0.0001)
      (Variables|Default|SettmpTransform (Transformation|GetWorldTransform (Variables|Default|GetArrow)))
      (else
        (Variables|Default|SettmpTransform (Math|Transform|MakeTransform FromLocation (Math|Rotator|FindLookatRotation FromLocation TargetLocation)))))
    (if (Math|Vector|Equal(Vector) TargetLocation "0, 0, 0" 0.0001)
      ;[1 1 1] 直接用当前旋转方向发射子弹
      (Game|SpawnActorfromClass (Class|SWeaponBaseBP|GetProjectileClass) (Math|Transform|MakeTransform (.Location (Math|Transform|BreakTransform (Variables|Default|GettmpTransform))) (.Rotation (Math|Transform|BreakTransform (Variables|Default|GettmpTransform))) (.Scale (Math|Transform|BreakTransform (Variables|Default|GettmpTransform)))) "AlwaysSpawn" self (Variables|Default|GetInstigator))
      (Variables|Default|SetShootTick (+ (Variables|Default|GettmNow) (Math|Timespan|MakeTimespan 0 0 0 0 (Class|SWeaponBaseBP|GetShootInterval))))
      (else
        ;[1 1 1] 根据传入的目标位置，算出起始旋转方向，然后在发射子弹
        (Game|SpawnActorfromClass (Class|SWeaponBaseBP|GetProjectileClass) (Math|Transform|MakeTransform (.Location (Math|Transform|BreakTransform (Variables|Default|GettmpTransform))) (Math|Rotator|FindLookatRotation (.Location (Math|Transform|BreakTransform (Variables|Default|GettmpTransform))) TargetLocation) (.Scale (Math|Transform|BreakTransform (Variables|Default|GettmpTransform)))) "AlwaysSpawn" self (Variables|Default|GetInstigator))
        (Variables|Default|SetShootTick (+ (Variables|Default|GettmNow) (Math|Timespan|MakeTimespan 0 0 0 0 (Class|SWeaponBaseBP|GetShootInterval))))))))

(fn ConstructionScript)