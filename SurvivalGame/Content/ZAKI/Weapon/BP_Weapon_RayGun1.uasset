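; BP_Weapon_RayGun1 is a hitscan gun that deals instant point damage to whatever its shot hits.
; Fire forwards to a ray-shoot event that traces by object type from the Arrow component to the target location, ignoring the caster.
; Characters take damage only if their Force ID differs from the caster's, while other hit actors always take it.
; Debug trace drawing and hit or miss prints are left on.
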(event Custom|CustomEvent_RayShoot
  (params (FromLocation :type Vector) (Rotator :type Rotator) (Range :type Float%20%28single-precision%29) (TargetLocation :type Vector) (Caster :type Pawn%20Object%20Reference))
  (bind (_outhit _returnvalue) (Collision|LineTraceForObjects (Transformation|GetWorldLocation (Variables|Default|GetArrow)) TargetLocation (Utilities|Array|MakeArray "ObjectTypeQuery1" "ObjectTypeQuery2" "ObjectTypeQuery3" "ObjectTypeQuery7" "ObjectTypeQuery4") false (Utilities|Array|MakeArray Caster) "ForDuration"))
  (if _returnvalue
    (Development|PrintString (Utilities|GetDisplayName (.HitActor (Collision|BreakHitResult _outhit))))
    (Utilities|IsValid (.HitActor (Collision|BreakHitResult _outhit))
      (:Is%20Valid
        (bind _assbase_character (Utilities|Casting|CastToSBaseCharacter (.HitActor (Collision|BreakHitResult _outhit)))
          (:then
            (bind _assbase_character_2 (Utilities|Casting|CastToSBaseCharacter Caster))
            (if (!= (Class|SBaseCharacter|GetForceID _assbase_character_2) (Class|SBaseCharacter|GetForceID _assbase_character))
              (Game|Damage|ApplyPointDamage (.HitActor (Collision|BreakHitResult _outhit)) (Class|SWeaponBaseBP|GetDamagePreHit) (.Location (Collision|BreakHitResult _outhit)) _outhit (Game|GetInstigatorController) (Game|GetInstigator) "/Game/Base/DmgType_InstantWeapon.DmgType_InstantWeapon_C" :!label _label)))
          (:CastFailed
            (goto _label)))))
    (else
      (Development|PrintString "shoot nothing"))))

(event EventBeginPlay)

(event Collision|EventActorBeginOverlap
  (params (OtherActor :type Actor%20Object%20Reference)))

(event EventTick
  (params (DeltaSeconds :type Float%20%28single-precision%29)))

(event EventFire
  (params (FromLocation :type Vector%20%28by%20ref%29) (Rotator :type Rotator%20%28by%20ref%29) (Range :type Float%20%28single-precision%29) (TargetLocation :type Vector%20%28by%20ref%29) (Caster :type Pawn%20Object%20Reference))
  (CallFunction|CustomEventRayShoot FromLocation Rotator Range TargetLocation Caster))

(fn ConstructionScript)