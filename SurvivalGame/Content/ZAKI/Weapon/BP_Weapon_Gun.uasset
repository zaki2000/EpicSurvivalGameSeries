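; Gun weapon actor that spawns projectiles on demand through a rate-limited fire function.
; FireOnce enforces a minimum interval via timestamps and uses the passed transform, or the Arrow component's when that is default.
; Given a target, it combines that rotation with a look-at rotation but spawns at world origin instead of the muzzle location.
; RandomFireRotator adds random per-axis spread; shot sound calls are disconnected.
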(event EventBeginPlay)

(event Collision|EventActorBeginOverlap
  (params (OtherActor :type Actor%20Object%20Reference)))

(event EventTick
  (params (DeltaSeconds :type Float%20%28single-precision%29)))

(fn ConstructionScript)

(fn FireOnce
  (params (FireTransform :type Transform) (EndVector :type Vector))
  (bind _output_get (LocalVariables|SettmNow (Math|DateTime|Now)))
  (if (>= _output_get (Variables|Default|GetShootTick))
    (if (== FireTransform (Math|Transform|MakeTransform "0, 0, 0"))
      (LocalVariables|SettmpTransform (Transformation|GetWorldTransform (Variables|Default|GetArrow)))
      (else
        (LocalVariables|SettmpTransform FireTransform)))
    (if (Math|Vector|Equal(Vector) EndVector "0, 0, 0" 0.0001)
      ;[1 1 1] 直接用当前旋转方向发射子弹
      (Game|SpawnActorfromClass (Variables|Default|GetProjectileClass) (Math|Transform|MakeTransform (.Location (Math|Transform|BreakTransform (LocalVariables|GettmpTransform))) (CallFunction|RandomFireRotator (.Rotation (Math|Transform|BreakTransform (LocalVariables|GettmpTransform))) (Variables|Default|GetRandomRotation)) (.Scale (Math|Transform|BreakTransform (LocalVariables|GettmpTransform)))) "AlwaysSpawn" self 0)
      (Variables|Default|SetShootTick (+ (LocalVariables|GettmNow) (Math|Timespan|MakeTimespan 0 0 0 0 (Variables|Default|GetMinShootInterval_MS))))
      (else
        ;[1 1 1] 根据传入的目标位置，算出起始旋转方向，然后在发射子弹
        (Game|SpawnActorfromClass (Variables|Default|GetProjectileClass) (Math|Transform|MakeTransform "0, 0, 0" (CallFunction|RandomFireRotator (Math|Rotator|CombineRotators (.Rotation (Math|Transform|BreakTransform (LocalVariables|GettmpTransform))) (Math|Rotator|FindLookatRotation (.Location (Math|Transform|BreakTransform (LocalVariables|GettmpTransform))) EndVector)) (Variables|Default|GetRandomRotation))) "AlwaysSpawn" self 0)
        (Variables|Default|SetShootTick (+ (LocalVariables|GettmNow) (Math|Timespan|MakeTimespan 0 0 0 0 (Variables|Default|GetMinShootInterval_MS))))))))

(fn RandomFireRotator
  (params (Input :type Rotator) (Random :type Rotator))
  (bind (_roll _pitch _yaw) (Math|Rotator|BreakRotator Random))
  (bind (_roll_2 _pitch_2 _yaw_2) (Math|Rotator|BreakRotator Input))
  (if (Math|Rotator|Equal(Rotator) Random "0, 0, 0" 0.0001)
    (return Input)
    (else
      (bind _result (Math|Float|NegateFloat _roll)
        (:%20%20
          (bind _result_2 (Math|Float|NegateFloat _pitch)
            (:%20%20
              (bind _result_3 (Math|Float|NegateFloat _yaw)
                (:%20%20
                  (return (Math|Rotator|MakeRotator (+ (Math|Random|RandomFloatinRange _result _roll) _roll_2) (+ (Math|Random|RandomFloatinRange _result_2 _pitch) _pitch_2) (+ (Math|Random|RandomFloatinRange _result_3 _yaw) _yaw_2))))))))))))