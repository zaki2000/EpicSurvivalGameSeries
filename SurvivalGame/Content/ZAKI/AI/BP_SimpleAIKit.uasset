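; BP_SimpleAIKit is a reusable setup Blueprint that starts Behavior Tree AI for a pawn that chases and shoots.
; InitlizeAI validates the AI controller and pawn, applies the Blackboard, seeds it and runs the Behavior Tree, returning false if either reference is invalid.
; InitlizeBlackBoard caches the references and copies tuning variables into keys for self, home location, chase and shoot settings, and waypoint class.
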(event EventBeginPlay)

(event EventTick
  (params (DeltaSeconds :type Float%20%28single-precision%29)))

(fn InitlizeAI
  (params (AIController :type AI%20Controller%20Object%20Reference) (Pawn :type Pawn%20Object%20Reference))
  (Utilities|IsValid AIController
    (:Is%20Valid
      (Utilities|IsValid Pawn
        (:Is%20Valid
          (bind _blackboardcomponent (Class|AIController|UseBlackboard AIController (Variables|Default|GetBlackBoard)))
          (CallFunction|InitlizeBlackBoard AIController Pawn _blackboardcomponent)
          (bind _returnvalue (AI|RunBehaviorTree AIController (Variables|Default|GetBTTree)))
          (return _returnvalue))
        (:Is%20Not%20Valid
          _)))
    (:Is%20Not%20Valid
      _))
  (return false))

(fn InitlizeBlackBoard
  (params (AIController :type AI%20Controller%20Object%20Reference) (Pawn :type Pawn%20Object%20Reference) (BB :type Blackboard%20Component%20Object%20Reference))
  (LocalVariables|SetmyController AIController)
  (LocalVariables|SetmyPawn Pawn)
  (LocalVariables|SetmyBB BB)
  (AI|Components|Blackboard|SetValueasObject (LocalVariables|GetmyBB) (LocalVariables|GetmySelf) (LocalVariables|GetmyPawn))
  (AI|Components|Blackboard|SetValueasFloat (LocalVariables|GetmyBB) (LocalVariables|GetmyChaseRange) (Variables|Default|GetChaseRange))
  (AI|Components|Blackboard|SetValueasVector (LocalVariables|GetmyBB) (LocalVariables|GetmyHome) (Transformation|GetActorLocation (LocalVariables|GetmyPawn)))
  (AI|Components|Blackboard|SetValueasFloat (LocalVariables|GetmyBB) (LocalVariables|GetmyChaseStopDistance) (Variables|Default|GetChaseStopDistance))
  (AI|Components|Blackboard|SetValueasFloat (LocalVariables|GetmyBB) (LocalVariables|GetmyShootDistance) (Variables|Default|GetShootDistance))
  (AI|Components|Blackboard|SetValueasFloat (LocalVariables|GetmyBB) (LocalVariables|GetmyShootInterval) (Variables|Default|GetShootInterval))
  (Class|BlackboardComponent|SetValueasClass (LocalVariables|GetmyBB) (LocalVariables|GetmyWayPointClass) (Variables|Default|GetWayPointClass)))