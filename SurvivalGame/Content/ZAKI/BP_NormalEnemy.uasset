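; BP_NormalEnemy is a standard enemy character that fires a weapon on command and changes its collision when its shields break.
; The use-skill command event calls UseCurrentSkill, which casts the Weapon child actor to SWeaponBase_BP and fires it from the enemy's transform toward the target location.
; When all shields are broken, the capsule and mesh are set to block the custom GameTraceChannel1 collision channel.
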(event EventBeginPlay)

(event EventOnEventAllShieldsBroken
  (Collision|SetCollisionResponsetoChannel (Variables|Default|GetCapsuleComponent) "ECC_GameTraceChannel1" "ECR_Block")
  (Collision|SetCollisionResponsetoChannel (Variables|Character|GetMesh) "ECC_GameTraceChannel1" "ECR_Block"))

(event EventOnCommondUseCurrentSkill
  (params (TargetLocation :type Vector%20%28by%20ref%29))
  (CallFunction|UseCurrentSkill TargetLocation))

(event EventTick
  (params (DeltaSeconds :type Float%20%28single-precision%29)))

(fn ConstructionScript
  (|CallParentFunction))

(fn UseCurrentSkill
  (params (TargetLocation :type Vector))
  (bind _self self)
  (bind _weapon (Variables|Default|GetWeapon))
  (bind _returnvalue (Transformation|GetActorTransform _self))
  (bind (_location _rotation) (Math|Transform|BreakTransform _returnvalue))
  (Utilities|IsValid _weapon
    (:Is%20Valid
      (bind _assweapon_base_bp (Utilities|Casting|CastToSWeaponBase_BP (Variables|/Script/Engine.ChildActorComponent|GetChildActor _weapon)))
      (Class|SWeaponBaseBP|Fire _assweapon_base_bp _location _rotation 0.0 TargetLocation))))